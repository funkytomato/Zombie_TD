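; Master melee weapon Blueprint, apparently a base for melee weapons, with durability that wears down on each use.
; Swing flags the weapon as attacking, reduces its clamped Health by a fixed step and enables query and physics collision.
; At zero Health it is marked broken and destroys itself after a short lifespan.
; Collision overlap casts to ZombieNPC_BP but applies no damage yet, and the hit event is empty.
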(event OnComponentHit(Collision)
  (params (HitComponent :type Primitive%20Component%20Object%20Reference) (OtherActor :type Actor%20Object%20Reference) (OtherComp :type Primitive%20Component%20Object%20Reference) (NormalImpulse :type Vector :default "0, 0, 0") (Hit :type Hit%20Result%20Structure%20%28by%20ref%29)))

(event OnComponentBeginOverlap(Collision)
  (params (OverlappedComponent :type Primitive%20Component%20Object%20Reference) (OtherActor :type Actor%20Object%20Reference) (OtherComp :type Primitive%20Component%20Object%20Reference) (OtherBodyIndex :type Integer) (bFromSweep :type Boolean) (SweepResult :type Hit%20Result%20Structure%20%28by%20ref%29))
  (Utilities|Casting|CastToZombieNPC_BP OtherActor))

(event Custom|Swing
  ;[1 1 1] Use Bat, Appy Wear and Tear, Inflict Damage
  (Variables|Default|SetIsAttacking? true)
  (CallFunction|ApplyWearandTear)
  (Collision|SetCollisionEnabled (Variables|Default|GetCollision) "QueryAndPhysics"))

(event Custom|ApplyWearAndTear
  ;[1 1 1] Apply Wear and Tear to Weapon
  (bind _output_get (Variables|Default|SetHealth (Math|Float|Clamp(Float) (- (Variables|Default|GetHealth) 0.1))))
  ;[1 1 1] Destroy Weapon if Broken
  (bind _output_get_2 (Variables|Default|SetisBroken? (<= _output_get 0.0)))
  (if _output_get_2
    (CallFunction|Broken)))

(event Custom|Broken
  ;[1 1 1] Is Broken, Destroy
  (Actor|SetLifeSpan 1.0))

(fn ConstructionScript
  (|CallParentFunction))