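; MasterGunWeapon_BP is a gun weapon Blueprint, named as the master for guns, that stubs out shooting and clip ammo handling.
; Its Shoot event is empty, and the construction script does nothing.
; Unconnected nodes sketch subtracting ShotCount from a clamped ClipCount and setting ReloadRequired when the clip is empty, but none of them run.
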(event Custom|Shoot)

(fn ConstructionScript)