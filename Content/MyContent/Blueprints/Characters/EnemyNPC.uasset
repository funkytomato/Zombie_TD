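; Enemy NPC character Blueprint, largely a skeleton that defers BeginPlay and AnyDamage to its parent class.
; It declares events for hits, server and client damage, ragdoll, and death variants by direction, weapon and stance, all with empty bodies.
; DecreaseStamina and IncreaseHealth are unfinished: their clamp results go unused, and the Exhausted call in DecreaseStamina is never reached.
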(fn ConstructionScript)

(event Custom|DeathFromRear
  ;[1 1 1] Death Animations
  ;;[1 1 1] Death from behind
)

(event Custom|DeathFromFront
  ;[1 1 1] Death Animations
  ;;[1 1 1] Death from Front
)

(event Custom|DeathFromIronSights
  ;[1 1 1] Death Animations
  ;;[1 1 1] Death from Ironsights
)

(event Custom|ProneDeath
  ;[1 1 1] Death Animations
  ;;[1 1 1] Death whilst Prone
)

(event Custom|ReactDeath
  ;[1 1 1] Death Animations
  ;;[1 1 1] Standing Reaction Death
)

(event Custom|DeathBySword
  ;[1 1 1] Death Animations
  ;;[1 1 1] Death by Sword
)

(event Custom|PistolWhipped
  ;[1 1 1] Death Animations
  ;;[1 1 1] PistolWhipped
)

(event Custom|OnDeath
  ;[1 1 1] OnDeath
)

(event Custom|Headshot
  ;[1 1 1] Death Animations
  ;;[1 1 1] Death by Headshot
)

(event Custom|DeathFromRight
  ;[1 1 1] Death Animations
  ;;[1 1 1] Death from the Right
)

(event Custom|DamageOnServer
  (params (Damage :type Float%20%28single-precision%29))
  ;[1 1 1] Taking Damage and KnockedOut
  ;;[1 1 1] Replicate
)

(event Custom|DamageOnClient
  (params (Damage :type Float%20%28single-precision%29))
  ;[1 1 1] Taking Damage and KnockedOut
)

(event Custom|Ragdoll
  ;[1 1 1] Taking Damage and KnockedOut
  ;;[1 1 1] Ragdoll
)

(event Collision|EventHit
  (params (MyComp :type Primitive%20Component%20Object%20Reference) (Other :type Actor%20Object%20Reference) (OtherComp :type Primitive%20Component%20Object%20Reference) (bSelfMoved :type Boolean) (HitLocation :type Vector :default "0, 0, 0") (HitNormal :type Vector :default "0, 0, 0") (NormalImpulse :type Vector :default "0, 0, 0") (Hit :type Hit%20Result%20Structure%20%28by%20ref%29)))

(event Game|Damage|EventAnyDamage
  (params (Damage :type Float%20%28single-precision%29) (DamageType :type Damage%20Type%20Object%20Reference) (InstigatedBy :type Controller%20Object%20Reference) (DamageCauser :type Actor%20Object%20Reference))
  ;[1 1 1] Taking Damage and KnockedOut
  ;;[1 1 1] Replicate
  (|CallParentFunction Damage DamageType InstigatedBy DamageCauser))

(event EventBeginPlay
  ;[1 1 1] BeginPlay - Startup
  (|CallParentFunction))